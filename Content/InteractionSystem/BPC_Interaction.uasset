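; Actor component that lets its owner detect interactable actors ahead of it and interact with them.
; A looping timer runs a short forward sphere trace, with debug drawing, and stores hits implementing BPI_Interaction as the target.
; The target's LookAtMessage feeds the player HUD's interaction widget, which is cleared when no target is found.
; IA_Interact calls InteractWith on the target's BPC_ItemData component, passing the owner.
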(event Custom|BeginInteraction
  (Utilities|Time|SetTimerbyEvent (delegate Custom|UpdateInteraction) 0.2 true))

(event Custom|UpdateInteraction
  (CallFunction|InteractionTrace))

(event Input|EnhancedActionEvents|EnhancedInputActionIA_Interact
  (params (ActionValue :type Boolean) (ElapsedSeconds :type Float%20%28double-precision%29) (TriggeredSeconds :type Float%20%28double-precision%29) (InputAction :type Input%20Action%20Object%20Reference :default "/Game/Variant_SideScroller/Input/Actions/IA_Interact.IA_Interact"))
  (:Started
    (bind _targetactor (Variables|Default|GetTargetActor)
      (:then
        (Utilities|IsValid (Actor|GetComponentbyClass _targetactor "/Game/InventorySystem/ItemData/BPC_ItemData.BPC_ItemData_C")
          (:Is%20Valid
            (Default|Interactwith (Actor|GetComponentbyClass _targetactor "/Game/InventorySystem/ItemData/BPC_ItemData.BPC_ItemData_C") (Components|GetOwner)))))
      (:else))))

(event EventBeginPlay
  (CallFunction|BeginInteraction))

(fn GetInteractionUI
  (bind _asbp_third_person_player_controller (Utilities|Casting|CastToBP_ThirdPersonPlayerController (Game|GetPlayerController 0)))
  (return (Variables|/Game/Player/UI/WB_PlayerHUD.WB_PlayerHUD_C|GetWB_InteractionUI (Variables|/Game/ThirdPerson/Blueprints/BP_ThirdPersonPlayerController.BP_ThirdPersonPlayerController_C|GetWB_PlayerHUD _asbp_third_person_player_controller))))

(fn InteractionTrace
  (bind _returnvalue (Components|GetOwner))
  (bind _returnvalue_2 (Transformation|GetActorLocation _returnvalue))
  (bind (_outhit _returnvalue_3) (Collision|SphereTraceByChannel _returnvalue_2 (+ _returnvalue_2 (* (Transformation|GetActorForwardVector _returnvalue) 1e+02)) 7e+01 "TraceTypeQuery3" false 0 "ForOneFrame"))
  (if _returnvalue_3
    (if (Utilities|DoesObjectImplementInterface (.HitActor (Collision|BreakHitResult _outhit)) "/Game/InteractionSystem/BPI_Interaction.BPI_Interaction_C")
      (bind _output_get (Variables|Default|SetTargetActor (.HitActor (Collision|BreakHitResult _outhit))))
      (bind _message (Class|BPIInteraction|Lookat(Message) _output_get))
      (Default|SetMessage (CallFunction|GetInteractionUI) _message)
      (else
        (Variables|Default|SetTargetActor 0)
        (Default|SetMessage (CallFunction|GetInteractionUI))))
    (else
      (Variables|Default|SetTargetActor 0)
      (Default|SetMessage (CallFunction|GetInteractionUI)))))