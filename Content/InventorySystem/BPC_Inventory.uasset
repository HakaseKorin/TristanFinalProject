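; Inventory component that stores items as ID and quantity pairs in a fixed-size slot array, sized on BeginPlay.
; PickUp relies on helpers for finding matching stacks below their DT_ItemData limit or empty slots, and plays the item's pickup sound at the owner.
; Other functions total an item's quantity, remove it one unit at a time, clearing the ID of emptied slots, and print contents.
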(event EventBeginPlay
  (Utilities|Array|Resize (Variables|Default|GetItemSlots) (Variables|Default|GetInventorySize)))

(fn PrintInventory
  (for (_array_element _array_index) (Variables|Default|GetItemSlots)
    (Development|PrintString (Utilities|String|Append (Utilities|String|ToString(Integer) _array_index) "" (Utilities|String|ToString(Name) (.ItemID (Utilities|Struct|BreakS_ItemSlot _array_element))) "" (Utilities|String|ToString(Integer) (.ItemQuantity (Utilities|Struct|BreakS_ItemSlot _array_element)))))))

(fn PickUp
  (params (ItemID :type Name) (ItemQuantity :type Integer))
  (bind (_success _index) (CallFunction|AnySlotAvaliable))
  (bind _output_get (LocalVariables|SetLocal_ItemQuantity ItemQuantity))
  (while (and (> _output_get 0) (not (LocalVariables|GetLocal_IsFull)))
    (bind _index_2 (CallFunction|FindMatchingSlot ItemID))
    (if true
      (CallFunction|AddtoSlot _index_2)
      (Math|Integer|DecrementInt (LocalVariables|GetLocal_ItemQuantity) :!label _label
        (:%20%20
          (CallFunction|PlayItemSFX (Utilities|Struct|BreakS_ItemSFX (CallFunction|GetItemSFX ItemID)))
          (return true 0)))
      (elif _success
        (CallFunction|AddtoNewSlot ItemID 1 _index)
        (goto _label)
        (else
          (LocalVariables|SetLocal_IsFull true)))))
  (return (not (LocalVariables|GetLocal_IsFull)) (LocalVariables|GetLocal_ItemQuantity)))

(fn FindMatchingSlot
  (params (ItemID :type Name))
  (for (_array_element _array_index) (Variables|Default|GetItemSlots)
    (if (and (== ItemID (.ItemID (Utilities|Struct|BreakS_ItemSlot _array_element))) (< (.ItemQuantity (Utilities|Struct|BreakS_ItemSlot _array_element)) (.Quantity (Utilities|Struct|BreakS_ItemInfo (CallFunction|GetItemData ItemID)))))
      (return true _array_index)))
  (return false -1))

(fn GetItemData
  (params (ItemID :type Name))
  (bind _returnvalue (Utilities|GetDataTableRow "/Game/InventorySystem/ItemData/DT_ItemData.DT_ItemData" ItemID)
    (:then
      (return _returnvalue))))

(fn AddtoSlot
  (params (Index :type Integer) (ItemQuantity :type Integer))
  (bind _itemslots (Variables|Default|GetItemSlots))
  (bind _output (Utilities|Array|Get(acopy) _itemslots Index))
  (Utilities|Array|SetArrayElem (Variables|Default|GetItemSlots) Index (Utilities|Struct|MakeS_ItemSlot (.itemid _output) (+ (.itemquantity _output) ItemQuantity))))

(fn AnySlotAvaliable
  (for (_array_element _array_index) (Variables|Default|GetItemSlots)
    (if (== (.ItemQuantity (Utilities|Struct|BreakS_ItemSlot _array_element)) 0)
      (return true _array_index)))
  (return false -1))

(fn AddtoNewSlot
  (params (ItemID :type Name) (ItemQuantity :type Integer) (Index :type Integer))
  (Utilities|Array|SetArrayElem (Variables|Default|GetItemSlots) Index (Utilities|Struct|MakeS_ItemSlot ItemID ItemQuantity)))

(fn PlayItemSFX
  (params (Sound :type Sound%20Base%20Object%20Reference))
  (Audio|PlaySoundatLocation Sound (Transformation|GetActorLocation (Components|GetOwner)) "0, 0, 0" 1.0 1.0 0.0 0 0 0 0))

(fn GetItemSFX
  (params (ItemID :type Name))
  (return (Utilities|Struct|BreakS_ItemInfo (CallFunction|GetItemData ItemID))))

(fn RemovefromStack
  (params (Index :type Integer) (Quantity :type Integer))
  (bind _itemslots (Variables|Default|GetItemSlots))
  (bind _output (Utilities|Array|Get(acopy) _itemslots Index))
  (bind (_itemid _itemquantity) (Utilities|Struct|BreakS_ItemSlot _output))
  (bind _returnvalue (- _itemquantity Quantity))
  (Utilities|Struct|SetmembersinS_ItemSlot _output (Utilities|String|SelectName _itemid "None" (!= _returnvalue 0)) _returnvalue))

(fn GetTotalItemQuantity
  (params (Item%20ID :type Name))
  (for _array_element (Variables|Default|GetItemSlots)
    (if (== (.ItemID (Utilities|Struct|BreakS_ItemSlot _array_element)) Item%20ID)
      (LocalVariables|SetLocal_TotalQuantity (+ (.ItemQuantity (Utilities|Struct|BreakS_ItemSlot _array_element)) (LocalVariables|GetLocal_TotalQuantity)))))
  (return (LocalVariables|GetLocal_TotalQuantity)))

(fn RemoveItemfromInventory
  (params (ItemID :type Name) (ItemQuantity :type Integer))
  (bind _output_get (LocalVariables|SetLocal_ItemQuantity ItemQuantity))
  (while (> _output_get 0)
    (bind (_array_element _array_index) (Utilities|Array|ForEachLoopwithBreak (Variables|Default|GetItemSlots) :!label _label)
      (:LoopBody
        (if (== (Utilities|Struct|BreakS_ItemSlot _array_element) ItemID)
          (CallFunction|RemovefromStack _array_index 1)
          (Math|Integer|DecrementInt (LocalVariables|GetLocal_ItemQuantity)
            (:%20%20
              (goto _label Break)))))))
  (return))