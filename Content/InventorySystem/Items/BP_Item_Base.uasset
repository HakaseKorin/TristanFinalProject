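; Base inventory item actor that represents a pickup in the world, configured from a data table row.
; GetItemData looks up the row named by the table and row reference in its BPCItemData component.
; The construction script uses that row to set ItemMesh's static mesh and per-slot materials.
; LookAt returns a "Pick Up" prompt formatted with the item's name; the event graph has no active logic.
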(event EventBeginPlay)

(event Collision|EventActorBeginOverlap
  (params (OtherActor :type Actor%20Object%20Reference)))

(event EventTick
  (params (DeltaSeconds :type Float%20%28single-precision%29)))

(fn ConstructionScript
  (CallFunction|SetItemMesh)
  (CallFunction|SetItemMaterial))

(fn GetItemData
  (bind _bpc_itemdata (Variables|Default|GetBPC_ItemData))
  (bind _itemdata (Variables|/Game/InventorySystem/ItemData/BPC_ItemData.BPC_ItemData_C|GetItemData _bpc_itemdata))
  (bind _returnvalue (Utilities|GetDataTableRow (.datatable _itemdata) (.rowname _itemdata))
    (:then
      (return _returnvalue))))

(fn SetItemMesh
  (Components|StaticMesh|SetStaticMesh (Variables|Default|GetItemMesh) (Utilities|Struct|BreakS_ItemMeshInfo (.Mesh (Utilities|Struct|BreakS_ItemInfo (CallFunction|GetItemData))))))

(fn SetItemMaterial
  (for (_array_element _array_index) (.Materials (Utilities|Struct|BreakS_ItemMeshInfo (.Mesh (Utilities|Struct|BreakS_ItemInfo (CallFunction|GetItemData)))))
    (Rendering|Material|SetMaterial (Variables|Default|GetItemMesh) _array_index _array_element)))

(fn Lookat
  (return (Utilities|Text|FormatText "Pick Up {Item}" (.Name (Utilities|Struct|BreakS_ItemInfo (CallFunction|GetItemData))))))